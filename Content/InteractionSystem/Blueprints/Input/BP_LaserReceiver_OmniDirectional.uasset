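; Omnidirectional laser receiver that switches on while at least one laser is connected and off when none remain.
; TryAddLaser registers each laser once if it hits the Detector component, and RemoveLaser unregisters it and prints the remaining lasers' names.
; Tick polls the connected list, using two DoOnce gates that reset each other so the state change and LaserInGlass effect toggle only on transitions.
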(event `self.ReceiveTick`
  (params (DeltaSeconds :type "Float (single-precision)"))
  (bind _laseringlass (`self.LaserInGlass`))
  (if (> (`KismetArrayLibrary.Array_Length` (`self.ConnectedLasers`)) 0)
    (`/Engine/EditorBlueprintResources/StandardMacros.DoOnce` false :!label _label
      (:`Completed`
        (`self.Set State On`)
        (`ActorComponent.Activate` _laseringlass true)
        (goto _label_2 :!via `Reset`)))
    (else
      (`/Engine/EditorBlueprintResources/StandardMacros.DoOnce` false :!label _label_2
        (:`Completed`
          (`self.Set State Off`)
          (`ActorComponent.Deactivate` _laseringlass)
          (goto _label :!via `Reset`))))))

(event `/Game/InteractionSystem/Blueprints/LaserSystem/LaserInterface.RemoveLaser`
  (params (Laser :type "Actor Object Reference"))
  (bind _connectedlasers (`self.ConnectedLasers`))
  (`KismetArrayLibrary.Array_RemoveItem` _connectedlasers Laser)
  (for _array_element _connectedlasers
    (`KismetSystemLibrary.PrintString` (`KismetSystemLibrary.GetDisplayName` _array_element))))

(fn `TryAddLaser`
  (params (ComponentHit :type "ActorComponent Object Reference") (Laser :type "Actor Object Reference"))
  (returns (HitSuccesful :type Boolean))
  (bind _connectedlasers (`self.ConnectedLasers`))
  (if (== ComponentHit (`self.Detector`))
    (if (< (`KismetArrayLibrary.Array_Find` _connectedlasers Laser) 0)
      (`KismetArrayLibrary.Array_Add` _connectedlasers Laser))
    (return true)
    (else
      (return false))))

(fn `UserConstructionScript`
  (`parent.UserConstructionScript`))