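; A timed kiosk button for the interaction system that turns on when pressed and switches itself off after a countdown.
; Interacting while off resets the timer, updates state and sync, and starts CheckTime, which re-calls itself each second to count down on a TextRender.
; At zero it turns off, then restores the displayed delay a second later.
; UpdateLight swaps the button top's glow material to match the state.
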(event `self.ReceiveBeginPlay`)

(event `CheckTime`
  (`TextRenderComponent.K2_SetText` (`self.TextRender`) (`KismetTextLibrary.Conv_IntToText` (`self.TimeRemaining`)))
  (if (== (`self.TimeRemaining`) 0)
    (`self.Set State Off`)
    (`self.Update Light`)
    (`self.Sync State`)
    (`KismetSystemLibrary.Delay` 1.0)
    (bind _output_get (set `self.TimeRemaining` (`self.TimeDelay`)))
    (`TextRenderComponent.K2_SetText` (`self.TextRender`) (`KismetTextLibrary.Conv_IntToText` _output_get))
    (else
      (set `self.TimeRemaining` (- (`self.TimeRemaining`) 1))
      (`KismetSystemLibrary.Delay` 1.0)
      (`self.CheckTime`))))

(event `/Game/InteractionSystem/Core/BPI_Interaction.Interact With`
  (if (not (`self.State`))
    (set `self.TimeRemaining` (`self.TimeDelay`))
    (`self.Set State On`)
    (`self.Update Light`)
    (`self.Sync State`)
    (`self.CheckTime`)))

(fn `Update Light`
  (`PrimitiveComponent.SetMaterial` (`self.SM_Button_Top`) 0 (select `bool` (`self.State`) :`false` "/Game/InteractionSystem/Assets/Materials/Glow/MI_Glow_Off.MI_Glow_Off" :`true` "/Game/InteractionSystem/Assets/Materials/Glow/MI_Glow_On.MI_Glow_On" :!type "MaterialInterface Object Reference")))

(fn `UserConstructionScript`
  (`parent.UserConstructionScript`))