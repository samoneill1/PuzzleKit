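; BP_Input is the master Blueprint for interaction-system inputs that switch connected devices on and off.
; On BeginPlay, StartOn selects SetStateOn or SetStateOff, which stores State and loops through Connections calling On or Off on each device.
; A per-connection Invert flag reverses the signal, so one input can drive devices in opposite states.
; UpdateChildren is empty, and the fracture, item type and mesh getters return only defaults.
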(event `self.ReceiveBeginPlay`
  (if (`self.StartOn`)
    (`self.Set State On`)
    (set `self.State` true)
    (else
      (`self.Set State Off`)
      (set `self.State` false))))

(fn `Get Fracture Bool`
  (returns (IsFracture :type Boolean))
  (return false))

(fn `Get Item Type`
  (returns (`Item Type` :type "/Game/InteractionSystem/Core/E_ItemType Enum"))
  (return "NewEnumerator0"))

(fn `Get Mesh`
  (returns (Mesh :type "PrimitiveComponent Object Reference"))
  (return null))

(fn `Set State Off`
  (set `self.State` false)
  (for _array_element (`self.Connections`)
    (if (`.Invert_8_01B3B2A949047C48E4B5FEBB83D663A9` (break `/Game/InteractionSystem/Blueprints/Input/Master/Connection` _array_element))
      (`/Game/InteractionSystem/Blueprints/Connections/Master/BP_Connection.On` (break `/Game/InteractionSystem/Blueprints/Input/Master/Connection` _array_element))
      (else
        (`/Game/InteractionSystem/Blueprints/Connections/Master/BP_Connection.Off` (break `/Game/InteractionSystem/Blueprints/Input/Master/Connection` _array_element))))))

(fn `Set State On`
  (set `self.State` true)
  (for _array_element (`self.Connections`)
    (if (`.Invert_8_01B3B2A949047C48E4B5FEBB83D663A9` (break `/Game/InteractionSystem/Blueprints/Input/Master/Connection` _array_element))
      (`/Game/InteractionSystem/Blueprints/Connections/Master/BP_Connection.Off` (break `/Game/InteractionSystem/Blueprints/Input/Master/Connection` _array_element))
      (else
        (`/Game/InteractionSystem/Blueprints/Connections/Master/BP_Connection.On` (break `/Game/InteractionSystem/Blueprints/Input/Master/Connection` _array_element))))))

(fn `Update Children`
  (returns (`Array Element` :type "/Game/InteractionSystem/Blueprints/Connections/Master/BP_Connection Object Reference")))

(fn `UserConstructionScript`)