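; BP_Button is an interactable push-button input for the interaction system that toggles an on/off state.
; Interacting plays a timeline that dips the button top and, on its Button Press event, flips the state via SetStateOn or SetStateOff.
; The top's material shows the state, which is then sent to every InputSync entry.
; Incoming SyncInputState updates state and material without re-broadcasting.
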(event `self.ReceiveBeginPlay`
  (`self.Update Light`))

(event `/Game/InteractionSystem/Core/BPI_Interaction.Interact With`
  (bind (_direction _alpha) (`Timeline|Timeline_ButtonAnimation` :!via `PlayFromStart`)
    (:`Update`
      (`SceneComponent.K2_SetRelativeLocation` (`self.SM_Button_Top`) (`KismetMathLibrary.VLerp` (0.0 0.0 0.0) (0.0 0.0 -5.0) _alpha) false false))
    (:`Button Press`
      (if (`self.State`)
        (`self.Set State Off`)
        (else
          (`self.Set State On`)))
      (`self.Update Light`)
      (`self.Sync State`))))

(event `/Game/InteractionSystem/Core/BPI_Interaction.Sync Input State`
  (params (State :type Boolean))
  (set `self.State_0` State)
  (`self.Update Light`))

(fn `Get Fracture Bool`
  (returns (IsFracture :type Boolean))
  (return false))

(fn `Get Item Type`
  (returns (`Item Type` :type "/Game/InteractionSystem/Core/E_ItemType Enum"))
  (return "NewEnumerator0"))

(fn `Get Mesh`
  (returns (Mesh :type "PrimitiveComponent Object Reference"))
  (return null))

(fn `Set State On`
  (`parent.Set State On`))

(fn `Sync State`
  (for _array_element (`self.Input Sync`)
    (message `/Game/InteractionSystem/Core/BPI_Interaction.Sync Input State` _array_element (`self.State`))))

(fn `Update Light`
  (`PrimitiveComponent.SetMaterial` (`self.SM_Button_Top`) 0 (select `bool` (`self.State`) :`false` "/Game/InteractionSystem/Assets/Materials/ProcGrid/MI_ProcGrid_OffLines.MI_ProcGrid_OffLines" :`true` "/Game/InteractionSystem/Assets/Materials/ProcGrid/MI_ProcGrid_OnLines.MI_ProcGrid_OnLines" :!type "MaterialInterface Object Reference")))

(fn `UserConstructionScript`)