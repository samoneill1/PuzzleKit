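; A directional laser receiver input for the interaction system, which turns on while at least one laser is connected.
; TryAddLaser accepts only hits on the Plane component, registering each laser once, and RemoveLaser unregisters it, printing a message on failure.
; Tick checks the connected list, using two mutually resetting DoOnce nodes to set the on/off state and swap the Plane's grid-line material only on transitions.
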(event `self.ReceiveTick`
  (params (DeltaSeconds :type "Float (single-precision)"))
  (bind _plane (`self.Plane`))
  (if (> (`KismetArrayLibrary.Array_Length` (`self.ConnectedLasers`)) 0)
    (`/Engine/EditorBlueprintResources/StandardMacros.DoOnce` false :!label _label
      (:`Completed`
        (`self.Set State On`)
        (`PrimitiveComponent.SetMaterial` _plane 0 "/Game/InteractionSystem/Assets/Materials/ProcGrid/MI_ProcGrid_OnLines.MI_ProcGrid_OnLines")
        (goto _label_2 :!via `Reset`)))
    (else
      (`/Engine/EditorBlueprintResources/StandardMacros.DoOnce` false :!label _label_2
        (:`Completed`
          (`self.Set State Off`)
          (`PrimitiveComponent.SetMaterial` _plane 0 "/Game/InteractionSystem/Assets/Materials/ProcGrid/MI_ProcGrid_OffLines.MI_ProcGrid_OffLines")
          (goto _label :!via `Reset`))))))

(event `/Game/InteractionSystem/Blueprints/LaserSystem/LaserInterface.RemoveLaser`
  (params (Laser :type "Actor Object Reference"))
  (bind _returnvalue (`KismetArrayLibrary.Array_RemoveItem` (`self.ConnectedLasers`) Laser))
  (if (not _returnvalue)
    (`KismetSystemLibrary.PrintString` (`KismetStringLibrary.Concat_StrStr` (`KismetSystemLibrary.GetDisplayName` Laser) " not removed from " (`KismetSystemLibrary.GetDisplayName` self)))))

(fn `TryAddLaser`
  (params (ComponentHit :type "ActorComponent Object Reference") (Laser :type "Actor Object Reference") (HItResult :type "HitResult Structure"))
  (returns (HitSuccesful :type Boolean))
  (bind _connectedlasers (`self.ConnectedLasers`))
  (if (== ComponentHit (`self.Plane`))
    (if (< (`KismetArrayLibrary.Array_Find` _connectedlasers Laser) 0)
      (`KismetArrayLibrary.Array_Add` _connectedlasers Laser))
    (return true)
    (else
      (return false))))

(fn `UserConstructionScript`
  (`parent.UserConstructionScript`))