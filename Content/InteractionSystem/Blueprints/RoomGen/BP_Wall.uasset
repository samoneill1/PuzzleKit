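; BP_Wall is a procedural wall actor that builds tiled walls from a mesh in the construction script, with no runtime logic.
; It converts WallSize into tile counts per axis using TileSize.
; MakeWall then runs twice, spawning a grid of static mesh components for each horizontal axis.
; Each grid is centered horizontally on the actor and rotated around Z, so the two runs are perpendicular and rise upward from the origin.
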(fn `DistanceToTileCount`
  (params (Distance :type "Float (double-precision)"))
  (returns (TileCount :type "Float (double-precision)"))
  (return (`KismetMathLibrary.Conv_IntToDouble` (`KismetMathLibrary.FTrunc` (/ Distance (`self.TileSize`))))))

(fn `MakeWall`
  (params (WallCount :type "Float (double-precision)") (Height :type "Float (double-precision)") (Rotation :type "Float (double-precision)"))
  (locals (HeightCount :type Integer))
  ;[1 1 1] Walls: Vertical
  (for _index (range (+ (`KismetMathLibrary.FTrunc` (- Height 0.0)) 1))
    (set `local.HeightCount` _index)
    ;;[1 1 1] Floor: Horizontal
    (for _index_2 (range (+ (`KismetMathLibrary.FTrunc` (- WallCount 1.0)) 1))
      (bind _returnvalue (`AddComponent|NODE_AddStaticMeshComponent-0` :`RelativeTransform` (`KismetMathLibrary.MakeTransform` (`KismetMathLibrary.RotateAngleAxis` (- (`KismetMathLibrary.MakeVector` 0.0 (* _index_2 (`self.TileSize`)) (* (`local.HeightCount`) (`self.TileSize`))) (/ (`KismetMathLibrary.MakeVector` 0.0 (- (* WallCount (`self.TileSize`)) (`self.TileSize`))) 2.0)) Rotation (0.0 0.0 1.0)) (`KismetMathLibrary.MakeRotator` 0.0 0.0 Rotation))))
      (`StaticMeshComponent.SetStaticMesh` _returnvalue (`self.Mesh`)))))

(fn `UserConstructionScript`
  (locals (XSize :type "Float (double-precision)" :default 0.0) (YSize :type "Float (double-precision)" :default 0.0) (ZSize :type "Float (double-precision)" :default 0.0))
  (bind _zsize (`local.ZSize`))
  (bind (_returnvalue_x _returnvalue_y _returnvalue_z) (`KismetMathLibrary.BreakVector` (* (`self.WallSize`) 2.0)))
  (`|ExecutionSequence`
    (:`then_0`
      (set `local.XSize` (`self.DistanceToTileCount` _returnvalue_x))
      (set `local.YSize` (`self.DistanceToTileCount` _returnvalue_y))
      (set `local.ZSize` (`self.DistanceToTileCount` (/ _returnvalue_z 2.0))))
    (:`then_1`
      (`self.MakeWall` (`local.XSize`) _zsize 90.0))
    (:`then_2`
      (`self.MakeWall` (`local.YSize`) _zsize))))