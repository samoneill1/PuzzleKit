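; Procedural ceiling actor for room generation that tiles a static mesh across a rectangular area at construction time.
; The Construction Script doubles FloorSize and converts it to whole tile counts by TileSize, discarding remainders; ZSize is computed but not used.
; MakeFloor runs nested loops, adding one rotated static mesh component per tile, offset so the grid centers on the actor origin.
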(fn `DistanceToTileCount`
  (params (Distance :type "Float (double-precision)"))
  (returns (TileCount :type "Float (double-precision)"))
  (return (`KismetMathLibrary.Conv_IntToDouble` (`KismetMathLibrary.FTrunc` (/ Distance (`self.TileSize`))))))

(fn `MakeFloor`
  (params (XSize :type "Float (double-precision)") (YSize :type "Float (double-precision)"))
  (locals (VertCount :type Integer) (NewLocalVar :type "Vector Structure"))
  (bind _tilesize (`self.TileSize`))
  (bind _tilesize_2 (`self.TileSize`))
  ;[1 1 1] Floor: Vertical
  (for _index (range (+ (`KismetMathLibrary.FTrunc` (- YSize 1.0)) 1))
    (set `local.VertCount` _index)
    ;;[1 1 1] Floor: Horizontal
    (for _index_2 (range (+ (`KismetMathLibrary.FTrunc` (- XSize 1.0)) 1))
      (bind _returnvalue (`AddComponent|NODE_AddStaticMeshComponent-0` :`RelativeTransform` (`KismetMathLibrary.MakeTransform` (- (`KismetMathLibrary.MakeVector` (* _index_2 _tilesize) (* (`local.VertCount`) _tilesize)) (/ (- (`KismetMathLibrary.MakeVector` (* XSize _tilesize_2) (* YSize _tilesize_2)) (`KismetMathLibrary.MakeVector` _tilesize_2 _tilesize_2)) 2.0)) (struct :`Pitch` 90.0))))
      (`StaticMeshComponent.SetStaticMesh` _returnvalue (`self.Mesh`)))))

(fn `UserConstructionScript`
  (locals (XSize :type "Float (double-precision)" :default 0.0) (YSize :type "Float (double-precision)" :default 0.0) (ZSize :type "Float (double-precision)" :default 0.0))
  (bind (_returnvalue_x _returnvalue_y _returnvalue_z) (`KismetMathLibrary.BreakVector` (* (`self.FloorSize`) 2.0)))
  (`|ExecutionSequence`
    (:`then_0`
      (set `local.XSize` (`self.DistanceToTileCount` _returnvalue_x))
      (set `local.YSize` (`self.DistanceToTileCount` _returnvalue_y))
      (set `local.ZSize` (`self.DistanceToTileCount` _returnvalue_z)))
    (:`then_1`
      (`self.MakeFloor` (`local.XSize`) (`local.YSize`)))))