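; Laser emitter actor that fires a Niagara beam along its emission point's forward vector and connects it to receivers it hits.
; Each tick, UpdateBeam line-traces forward to set the beam end, using a fixed maximum distance on a miss.
; Hit actors receive add-laser messages; the accepting one is cached and notified of removal when the target changes or is lost.
; The beam end stays unchanged while the trace hits the cached receiver.
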(event `self.ReceiveTick`
  (params (DeltaSeconds :type "Float (single-precision)"))
  (`self.UpdateBeam`))

(fn `RemoveConnectedLaser`
  (bind _connectedreceiver (`self.ConnectedReceiver`))
  (`/Engine/EditorBlueprintResources/StandardMacros.IsValid` _connectedreceiver
    (:`Is Valid`
      (message `/Game/InteractionSystem/Blueprints/LaserSystem/LaserInterface.RemoveLaser` _connectedreceiver self)
      (set `self.ConnectedReceiver` null))))

(fn `TryAddLaser`
  (params (ComponentHit :type "ActorComponent Object Reference") (Laser :type "Actor Object Reference") (HItResult :type "HitResult Structure")))

(fn `UpdateBeam`
  (locals (NewLocalVar :type "Vector Structure" :default (0.0 0.0 0.0)))
  (bind _emissionpoint (`self.EmissionPoint`))
  (bind _laser_ns (`self.Laser_NS`))
  (bind _returnvalue (`SceneComponent.K2_GetComponentLocation` _emissionpoint))
  (bind _returnvalue_2 (+ _returnvalue (* (`SceneComponent.GetForwardVector` _emissionpoint) 100000.0)))
  (bind _outhit (`KismetSystemLibrary.LineTraceSingle` _returnvalue _returnvalue_2 "TraceTypeQuery3"))
  (bind (_bblockinghit _binitialoverlap _time _distance _location _impactpoint _normal _impactnormal _physmat _hitactor _hitcomponent) (`GameplayStatics.BreakHitResult` _outhit))
  (if _bblockinghit
    (if (not (== (`self.ConnectedReceiver`) _hitactor))
      (`self.RemoveConnectedLaser`)
      (`FXSystemComponent.SetVectorParameter` _laser_ns "BeamEndLocation" _location)
      (bind _hitsuccesful (message `/Game/InteractionSystem/Blueprints/LaserSystem/LaserInterface.TryAddLaser` _hitactor _hitcomponent self _outhit))
      (if _hitsuccesful
        (set `self.ConnectedReceiver` _hitactor)
        (else
          (`self.RemoveConnectedLaser` :!label _label))))
    (else
      (`FXSystemComponent.SetVectorParameter` _laser_ns "BeamEndLocation" _returnvalue_2)
      (goto _label))))

(fn `UserConstructionScript`
  (bind _emissionpoint (`self.EmissionPoint`))
  (bind _returnvalue (`SceneComponent.K2_GetComponentLocation` _emissionpoint))
  (`KismetSystemLibrary.LineTraceSingle` :`Start` _returnvalue :`End` (+ _returnvalue (* (`SceneComponent.GetForwardVector` _emissionpoint) 100000.0)) :`TraceChannel` "TraceTypeQuery3" :`DrawDebugType` "ForOneFrame")
  (`FXSystemComponent.SetVectorParameter` (`self.Laser_NS`) "BeamEndLocation" _returnvalue))