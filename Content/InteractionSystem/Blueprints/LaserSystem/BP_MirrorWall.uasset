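; Mirror wall actor in a laser system that reflects each incoming laser and passes it on to whatever the reflection hits.
; TryAddLaser stores impact point and normal per laser in maps and spawns a Niagara beam.
; Tick line-traces each reflection, mirroring the stored normal about the actor's right vector, and registers the wall as a laser on newly hit receivers.
; Lost targets and removed lasers send removal messages downstream, so beams can chain.
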(event `self.ReceiveTick`
  (params (DeltaSeconds :type "Float (single-precision)"))
  (bind _keys (`BlueprintMapLibrary.Map_Keys` (`self.LaserImpactPoints`)))
  (for _array_element _keys
    (`self.UpdateBeam` _array_element)))

(event `/Game/InteractionSystem/Blueprints/LaserSystem/LaserInterface.RemoveLaser`
  (params (Laser :type "Actor Object Reference"))
  (bind _laserparticlesystems (`self.LaserParticleSystems`))
  (message `/Game/InteractionSystem/Blueprints/LaserSystem/LaserInterface.RemoveLaser` (`BlueprintMapLibrary.Map_Find` (`self.ConnectedReceivers`) Laser) self)
  (`BlueprintMapLibrary.Map_Remove` (`self.LaserImpactPoints`) Laser)
  (`BlueprintMapLibrary.Map_Remove` (`self.LaserImpactNormals`) Laser)
  (`ActorComponent.K2_DestroyComponent` (`BlueprintMapLibrary.Map_Find` _laserparticlesystems Laser))
  (`BlueprintMapLibrary.Map_Remove` _laserparticlesystems Laser)
  (`BlueprintMapLibrary.Map_Remove` (`self.ConnectedReceivers`) Laser))

(fn `RemoveConnectedLaser`
  (params (Laser :type "Actor Object Reference"))
  (bind _connectedreceivers (`self.ConnectedReceivers`))
  (bind _value (`BlueprintMapLibrary.Map_Find` _connectedreceivers Laser))
  (`/Engine/EditorBlueprintResources/StandardMacros.IsValid` _value
    (:`Is Valid`
      (message `/Game/InteractionSystem/Blueprints/LaserSystem/LaserInterface.RemoveLaser` _value self)
      (`BlueprintMapLibrary.Map_Add` _connectedreceivers Laser))))

(fn `TryAddLaser`
  (params (ComponentHit :type "ActorComponent Object Reference") (Laser :type "Actor Object Reference") (HItResult :type "HitResult Structure"))
  (returns (HitSuccesful :type Boolean))
  (`BlueprintMapLibrary.Map_Add` (`self.LaserImpactPoints`) Laser HItResult_ImpactPoint)
  (`BlueprintMapLibrary.Map_Add` (`self.LaserImpactNormals`) Laser HItResult_Normal)
  (bind _returnvalue (`AddComponent|NODE_AddNiagaraComponent-0`))
  (`NiagaraComponent.SetAsset` _returnvalue "/Game/InteractionSystem/Blueprints/LaserSystem/LaserBeam_NS.LaserBeam_NS" true)
  (`BlueprintMapLibrary.Map_Add` (`self.LaserParticleSystems`) Laser _returnvalue)
  (return true))

(fn `UpdateBeam`
  (params (CurrentLaser :type "Actor Object Reference"))
  (locals (LocalCurrentLaser :type "Actor Object Reference"))
  (bind _value (`BlueprintMapLibrary.Map_Find` (`self.LaserParticleSystems`) (`local.LocalCurrentLaser`)))
  (bind _output_get (set `local.LocalCurrentLaser` CurrentLaser))
  (bind _value_2 (`BlueprintMapLibrary.Map_Find` (`self.LaserImpactPoints`) _output_get))
  (`SceneComponent.K2_SetWorldLocation` (`BlueprintMapLibrary.Map_Find` (`self.LaserParticleSystems`) (`local.LocalCurrentLaser`)) _value_2 false false)
  (bind _returnvalue (+ _value_2 (* (`KismetMathLibrary.GetReflectionVector` (`BlueprintMapLibrary.Map_Find` (`self.LaserImpactNormals`) _output_get) (`self.GetActorRightVector`)) 100000000.0)))
  (bind _outhit (`KismetSystemLibrary.LineTraceSingle` _value_2 _returnvalue "TraceTypeQuery3"))
  (bind (_bblockinghit _binitialoverlap _time _distance _location _impactpoint _normal _impactnormal _physmat _hitactor _hitcomponent) (`GameplayStatics.BreakHitResult` _outhit))
  (if _bblockinghit
    (if (not (== (`BlueprintMapLibrary.Map_Find` (`self.ConnectedReceivers`) (`local.LocalCurrentLaser`)) _hitactor))
      (`self.RemoveConnectedLaser` (`local.LocalCurrentLaser`))
      (`FXSystemComponent.SetVectorParameter` _value "BeamEndLocation" _location)
      (bind _hitsuccesful (message `/Game/InteractionSystem/Blueprints/LaserSystem/LaserInterface.TryAddLaser` _hitactor _hitcomponent self _outhit))
      (if _hitsuccesful
        (`BlueprintMapLibrary.Map_Add` (`self.ConnectedReceivers`) (`local.LocalCurrentLaser`) _hitactor)
        (else
          (`self.RemoveConnectedLaser` (`local.LocalCurrentLaser`) :!label _label))))
    (else
      (`FXSystemComponent.SetVectorParameter` _value "BeamEndLocation" _returnvalue)
      (goto _label))))

(fn `UserConstructionScript`)