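; A disappearing platform Blueprint that vanishes shortly after the player steps on it, then comes back.
; When a BP_FPS_Character begins overlapping the Box trigger, the Floor mesh changes material as a cue, then after a short delay is hidden and loses collision.
; Any actor ending overlap starts a second delay, after which the Floor's grid material, visibility and collision are restored.
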(event `self.Box.OnComponentBeginOverlap`
  (params (OverlappedComponent :type "PrimitiveComponent Object Reference") (OtherActor :type "Actor Object Reference") (OtherComp :type "PrimitiveComponent Object Reference") (OtherBodyIndex :type Integer) (bFromSweep :type Boolean) (SweepResult :type "HitResult Structure (by ref)"))
  (cast `/Game/InteractionSystem/Blueprints/Player/BP_FPS_Character` OtherActor)
  (`PrimitiveComponent.SetMaterial` (`self.floor`) 0 "/Game/InteractionSystem/Assets/Materials/Basic/M_Basic_Beige.M_Basic_Beige")
  (`KismetSystemLibrary.Delay` 0.9)
  (`SceneComponent.SetVisibility` (`self.floor`) false false)
  (`PrimitiveComponent.SetCollisionEnabled` (`self.floor`) "NoCollision"))

(event `self.Box.OnComponentEndOverlap`
  (params (OverlappedComponent :type "PrimitiveComponent Object Reference") (OtherActor :type "Actor Object Reference") (OtherComp :type "PrimitiveComponent Object Reference") (OtherBodyIndex :type Integer))
  (`KismetSystemLibrary.Delay` 1.5)
  (`PrimitiveComponent.SetMaterial` (`self.floor`) 0 "/Game/InteractionSystem/Assets/Materials/ProcGrid/MI_ProcGrid.MI_ProcGrid")
  (`SceneComponent.SetVisibility` (`self.floor`) true false)
  (`PrimitiveComponent.SetCollisionEnabled` (`self.floor`) "QueryAndPhysics"))

(fn `UserConstructionScript`)