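; Laser redirector item that, while at least one laser feeds into its mesh, emits its own beam from an emission point.
; TryAddLaser and RemoveLaser track incoming lasers, and Tick uses paired DoOnce nodes to toggle the Niagara beam effects.
; While powered, UpdateBeam line-traces forward each tick, setting the beam endpoint and handing itself between receivers through add/remove laser messages, which allows chaining.
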(event `self.ReceiveTick`
  (params (DeltaSeconds :type "Float (single-precision)"))
  (bind _laserns (`self.LaserNS`))
  (bind _laserinsphere_ns (`self.LaserInSphere_NS`))
  (if (> (`KismetArrayLibrary.Array_Length` (`self.ConnectedLasers`)) 0)
    (`|ExecutionSequence`
      (:`then_0`
        (`/Engine/EditorBlueprintResources/StandardMacros.DoOnce` false :!label _label
          (:`Completed`
            (`ActorComponent.Activate` _laserns true)
            (`ActorComponent.Activate` _laserinsphere_ns true)
            (goto _label_2 :!via `Reset`))))
      (:`then_1`
        (`self.UpdateBeam`)))
    (else
      (`/Engine/EditorBlueprintResources/StandardMacros.DoOnce` false :!label _label_2
        (:`Completed`
          (`ActorComponent.Deactivate` _laserns)
          (`ActorComponent.Deactivate` _laserinsphere_ns)
          (goto _label :!via `Reset`))))))

(event `/Game/InteractionSystem/Blueprints/LaserSystem/LaserInterface.RemoveLaser`
  (params (Laser :type "Actor Object Reference"))
  (`KismetArrayLibrary.Array_RemoveItem` (`self.ConnectedLasers`) Laser))

(fn `RemoveConnectedLaser`
  (bind _connectedreceiver (`self.ConnectedReceiver`))
  (`/Engine/EditorBlueprintResources/StandardMacros.IsValid` _connectedreceiver
    (:`Is Valid`
      (message `/Game/InteractionSystem/Blueprints/LaserSystem/LaserInterface.RemoveLaser` _connectedreceiver self)
      (set `self.ConnectedReceiver` null))))

(fn `TryAddLaser`
  (params (ComponentHit :type "ActorComponent Object Reference") (Laser :type "Actor Object Reference") (HItResult :type "HitResult Structure"))
  (returns (HitSuccesful :type Boolean))
  (if (== (`self.Mesh`) ComponentHit)
    (`KismetArrayLibrary.Array_Add` (`self.ConnectedLasers`) Laser)
    (return true)
    (else
      (return false))))

(fn `UpdateBeam`
  (locals (NewLocalVar :type "Vector Structure" :default (0.0 0.0 0.0)) (NewLocalVar_0 :type "Vector Structure"))
  (bind _emissionpoint (`self.EmissionPoint`))
  (bind _laser_end (`self.Laser_End`))
  (bind _laserns (`self.LaserNS`))
  (bind _returnvalue (`SceneComponent.K2_GetComponentLocation` _emissionpoint))
  (bind _returnvalue_2 (+ _returnvalue (* (`SceneComponent.GetForwardVector` _emissionpoint) 100000.0)))
  (bind _outhit (`KismetSystemLibrary.LineTraceSingle` _returnvalue _returnvalue_2 "TraceTypeQuery3"))
  (bind (_bblockinghit _binitialoverlap _time _distance _location _impactpoint _normal _impactnormal _physmat _hitactor _hitcomponent) (`GameplayStatics.BreakHitResult` _outhit))
  (if _bblockinghit
    (if (not (== (`self.ConnectedReceiver`) _hitactor))
      (`self.RemoveConnectedLaser`)
      (`FXSystemComponent.SetVectorParameter` _laserns "BeamEndLocation" _location)
      (bind _hitsuccesful (message `/Game/InteractionSystem/Blueprints/LaserSystem/LaserInterface.TryAddLaser` _hitactor _hitcomponent self _outhit))
      (if _hitsuccesful
        (set `self.ConnectedReceiver` _hitactor)
        (`ActorComponent.Deactivate` _laser_end)
        (else
          (`self.RemoveConnectedLaser`)
          (`ActorComponent.Activate` _laser_end false)
          (`FXSystemComponent.SetVectorParameter` _laser_end "BeamEndLocation" _location))))
    (else
      (`FXSystemComponent.SetVectorParameter` _laserns "BeamEndLocation" _returnvalue_2)
      (`self.RemoveConnectedLaser`))))

(fn `UpdateLaser`
  (bind _emissionpoint (`self.EmissionPoint`))
  (bind _connectedreceiver (`self.ConnectedReceiver`))
  (bind _laserns (`self.LaserNS`))
  (bind _returnvalue (`SceneComponent.K2_GetComponentLocation` _emissionpoint))
  (bind _returnvalue_2 (+ _returnvalue (* (`SceneComponent.GetForwardVector` _emissionpoint) 100000.0)))
  (bind _outhit (`KismetSystemLibrary.LineTraceSingle` _returnvalue _returnvalue_2 "TraceTypeQuery1" false (`|MakeArray` self :!type "Actor Object Reference")))
  (bind (_bblockinghit _binitialoverlap _time _distance _location _impactpoint _normal _impactnormal _physmat _hitactor _hitcomponent) (`GameplayStatics.BreakHitResult` _outhit))
  (if _bblockinghit
    (`FXSystemComponent.SetVectorParameter` _laserns "BeamEndLocation" _location)
    (bind _hitsuccesful (message `/Game/InteractionSystem/Blueprints/LaserSystem/LaserInterface.TryAddLaser` _hitactor _hitcomponent self _outhit))
    (if _hitsuccesful
      (set `self.ConnectedReceiver` null)
      (else
        (`/Engine/EditorBlueprintResources/StandardMacros.IsValid` _connectedreceiver :!label _label
          (:`Is Valid`
            (message `/Game/InteractionSystem/Blueprints/LaserSystem/LaserInterface.RemoveLaser` _connectedreceiver self)))))
    (else
      (`FXSystemComponent.SetVectorParameter` _laserns "BeamEndLocation" _returnvalue_2)
      (goto _label))))

(fn `UserConstructionScript`
  (`parent.UserConstructionScript`))