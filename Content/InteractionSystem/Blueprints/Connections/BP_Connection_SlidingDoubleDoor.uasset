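; Sliding double door connection for the interaction system that opens when switched On and closes when switched Off.
; On plays a timeline that lerps the two panels apart along local Y, and Off reverses it after calling the parent.
; The construction script feeds the RevealBlock's world location and bounds into a dynamic double-sided material shared by panels and frame pieces, defining a box region for the shader.
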(event `self.On`
  (`parent.On`)
  (bind (_direction _alpha) (`Timeline|Timeline_DoorAnimation` :!label _label)
    (:`Update`
      (`SceneComponent.K2_SetRelativeLocation` (`self.Mesh`) (`KismetMathLibrary.VLerp` (0.0 150.0 150.0) (0.0 300.0 150.0) _alpha) false false)
      (`SceneComponent.K2_SetRelativeLocation` (`self.DoorL`) (`KismetMathLibrary.VLerp` (0.0 -150.0 150.0) (0.0 -300.0 150.0) _alpha) false false))))

(event `self.Off`
  (`parent.Off`)
  (goto _label :!via `Reverse`))

(fn `Get Fracture Bool`
  (returns (IsFracture :type Boolean))
  (return false))

(fn `Get Item Type`
  (returns (`Item Type` :type "/Game/InteractionSystem/Core/E_ItemType Enum"))
  (return "NewEnumerator0"))

(fn `Get Mesh`
  (returns (Mesh :type "PrimitiveComponent Object Reference"))
  (return null))

(fn `UserConstructionScript`
  (bind _revealblock (`self.RevealBlock`))
  (`|ExecutionSequence`
    (:`then_0`
      (bind _returnvalue (`KismetMaterialLibrary.CreateDynamicMaterialInstance` "/Game/InteractionSystem/Assets/Materials/Master/M_Basic_BlockedDoubleSided.M_Basic_BlockedDoubleSided"))
      (`MaterialInstanceDynamic.SetVectorParameterValue` _returnvalue "BoxLocation" (`KismetMathLibrary.Conv_VectorToLinearColor` (`SceneComponent.K2_GetComponentLocation` _revealblock)))
      (`MaterialInstanceDynamic.SetVectorParameterValue` _returnvalue "BoxScale" (`KismetMathLibrary.Conv_VectorToLinearColor` (* (`.BoxExtent` (`KismetSystemLibrary.GetComponentBounds` _revealblock)) 2.0))))
    (:`then_1`
      (`PrimitiveComponent.SetMaterial` (`self.DoorL`) 0 _returnvalue)
      (`PrimitiveComponent.SetMaterial` (`self.Mesh`) 0 _returnvalue)
      (`PrimitiveComponent.SetMaterial` (`self.DoorFrameBottom`) 0 _returnvalue)
      (`PrimitiveComponent.SetMaterial` (`self.DoorFrameTop`) 0 _returnvalue))))