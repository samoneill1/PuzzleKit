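; AND gate for the interaction connection system that turns its connected objects on only while every input targeting it is on.
; Each On or Off event rechecks all inputs and updates one indicator light per input.
; Two cross-resetting DoOnce nodes forward only changes in the combined result to outgoing connections.
; The construction script previews lights, which BeginPlay replaces with one per actual input, resizing the mesh to fit.
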(event `self.ReceiveBeginPlay`
  (`parent.ReceiveBeginPlay`)
  (`self.SetUpLights`))

(event `self.On`
  (bind _returnstate (`self.CheckStates` :!label _label))
  (if _returnstate
    (`/Engine/EditorBlueprintResources/StandardMacros.DoOnce` false :!label _label_2
      (:`Completed`
        (`self.UpdateConnections` true)
        (goto _label_3 :!via `Reset`)))
    (else
      (`/Engine/EditorBlueprintResources/StandardMacros.DoOnce` false :!label _label_3
        (:`Completed`
          (`self.UpdateConnections` false)
          (goto _label_2 :!via `Reset`))))))

(event `self.Off`
  (goto _label))

(fn `CheckStates`
  (returns (ReturnState :type Boolean))
  (locals (LocalState :type Boolean))
  (set `local.LocalState` true)
  (for (_array_element _array_index) (`self.InputsTargettingMe`)
    (if (`/Game/InteractionSystem/Blueprints/Input/Master/BP_Input.State` _array_element)
      (bind _output (`|GetArrayItem` (`self.Lights`) _array_index))
      (`/Game/InteractionSystem/Blueprints/Connections/BP_IndicatorLight.On` _output)
      (else
        (set `local.LocalState` false)
        (`/Game/InteractionSystem/Blueprints/Connections/BP_IndicatorLight.Off` _output))))
  (return (`local.LocalState`)))

(fn `SetUpLights`
  (bind _inputstargettingme (`self.InputsTargettingMe`))
  (for _array_element (`self.TempLights`)
    (`self.K2_DestroyActor` _array_element))
  (for (_array_element_2 _array_index) _inputstargettingme
    (bind _returnvalue (`AddComponent|NODE_AddChildActorComponent-0` :`RelativeTransform` (`KismetMathLibrary.MakeTransform` (`KismetMathLibrary.MakeVector` 0.0 (- (`KismetMathLibrary.Conv_IntToDouble` (* _array_index 90)) (/ (* (- (`KismetArrayLibrary.Array_Length` _inputstargettingme) 1) 90) 2)) 75.0))))
    (`ChildActorComponent.SetChildActorClass` _returnvalue "/Game/InteractionSystem/Blueprints/Connections/BP_IndicatorLight.BP_IndicatorLight_C")
    (`KismetArrayLibrary.Array_Add` (`self.Lights`) (cast `/Game/InteractionSystem/Blueprints/Connections/BP_IndicatorLight` (`ChildActorComponent.ChildActor` _returnvalue) :!pure true))
    (`KismetSystemLibrary.PrintString` (`KismetSystemLibrary.GetDisplayName` _array_element_2)))
  (`SceneComponent.SetRelativeScale3D` (`self.Mesh`) (`KismetMathLibrary.MakeVector` 1.0 (/ (* (`KismetArrayLibrary.Array_Length` (`self.InputsTargettingMe`)) 100.0) 300.0) 0.5)))

(fn `SetUpTempLights`
  (params (Lights :type Integer))
  (bind _returnvalue (- Lights 1))
  (for _index (range (+ _returnvalue 1))
    (bind _returnvalue_2 (`AddComponent|NODE_AddChildActorComponent-1` :`RelativeTransform` (`KismetMathLibrary.MakeTransform` (`KismetMathLibrary.MakeVector` 0.0 (- (`KismetMathLibrary.Conv_IntToDouble` (* _index 90)) (/ (* _returnvalue 90) 2)) 75.0))))
    (`ChildActorComponent.SetChildActorClass` _returnvalue_2 "/Game/InteractionSystem/Blueprints/Connections/BP_IndicatorLight.BP_IndicatorLight_C")
    (`KismetArrayLibrary.Array_Add` (`self.TempLights`) (cast `/Game/InteractionSystem/Blueprints/Connections/BP_IndicatorLight` (`ChildActorComponent.ChildActor` _returnvalue_2) :!pure true)))
  (`SceneComponent.SetRelativeScale3D` (`self.Mesh`) (`KismetMathLibrary.MakeVector` 1.0 (/ (* Lights 100.0) 300.0) 0.5)))

(fn `UpdateConnections`
  (params (NewState :type Boolean))
  (for _array_element (`self.Connections`)
    (if NewState
      (`self.On` _array_element)
      (else
        (`self.Off` _array_element)))))

(fn `UserConstructionScript`
  (`parent.UserConstructionScript`)
  (`self.SetUpTempLights` (`self.TempLightCount`)))