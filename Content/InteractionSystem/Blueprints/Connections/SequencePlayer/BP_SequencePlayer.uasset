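; Interaction-system connection actor that drives a Level Sequence from On and Off events.
; BeginPlay creates the sequence player, setting looping, end pausing and input lock from PlayMode and EndBehaviour.
; Forward/Back flips direction on either event, Start/Stop resumes or pauses in the current direction, and Cut Scene plays on On with movement and look input disabled.
; Ping-Pong reverses on finish outside Cut Scene, whose finish handler is empty.
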(event `CustomEvent`)

(event `Ping-Pong`
  (bind _sequenceplayer (`LevelSequenceActor.SequencePlayer` (`self.SequencePlayerActor`)))
  (if (`MovieSceneSequencePlayer.IsReversed` _sequenceplayer)
    (`MovieSceneSequencePlayer.Play` _sequenceplayer)
    (else
      (`MovieSceneSequencePlayer.PlayReverse` _sequenceplayer))))

(event `self.ReceiveBeginPlay`
  (bind _endbehaviour (`self.EndBehaviour`))
  (bind _returnvalue (select `/Game/InteractionSystem/Blueprints/Connections/SequencePlayer/SequencePlayMode` (`self.PlayMode`) :`NewEnumerator2` true))
  (bind _sequenceplayer (`LevelSequenceActor.SequencePlayer` (`self.SequencePlayerActor`)))
  (`parent.ReceiveBeginPlay`)
  (bind _outactor (`LevelSequencePlayer.CreateLevelSequencePlayer` (`self.SequenceToPlay`) (make `MovieSceneSequencePlaybackSettings` false (make `MovieSceneSequenceLoopCount` (select `/Game/InteractionSystem/Blueprints/Connections/SequencePlayer/SequenceEndBehaviour` _endbehaviour :`NewEnumerator2` -1)) 1.0 0.0 false _returnvalue _returnvalue false false false "None" (select `/Game/InteractionSystem/Blueprints/Connections/SequencePlayer/SequenceEndBehaviour` _endbehaviour :`NewEnumerator0` true :`NewEnumerator1` true))))
  (set `self.SequencePlayerActor` _outactor)
  (`|ExecutionSequence`
    (:`then_0`
      (switch `/Game/InteractionSystem/Blueprints/Connections/SequencePlayer/SequencePlayMode` (`self.PlayMode`)
        (:`NewEnumerator0`
          (switch `/Game/InteractionSystem/Blueprints/Connections/SequencePlayer/SequenceEndBehaviour` (`self.EndBehaviour`) :!label _label
            (:`NewEnumerator1`
              (add `MovieSceneSequencePlayer.OnFinished` _sequenceplayer (delegate `Ping-Pong`)))))
        (:`NewEnumerator1`
          (goto _label))
        (:`NewEnumerator2`
          (add `MovieSceneSequencePlayer.OnFinished` _sequenceplayer (delegate `CustomEvent`)))))
    (:`then_1`
      (switch `/Game/InteractionSystem/Blueprints/Connections/SequencePlayer/SequencePlayMode` (`self.PlayMode`)
        (:`NewEnumerator0`
          (if (not (`self.State`))
            (`MovieSceneSequencePlayer.PlayReverse` _sequenceplayer)
            (`MovieSceneSequencePlayer.SetPlaybackPosition` _sequenceplayer (make `MovieSceneSequencePlaybackParams` (struct :`FrameNumber` (struct))))))))))

(event `self.On`
  (bind _sequenceplayer (`LevelSequenceActor.SequencePlayer` (`self.SequencePlayerActor`)))
  (bind _returnvalue (`MovieSceneSequencePlayer.IsReversed` _sequenceplayer))
  (`parent.On`)
  (`/Engine/EditorBlueprintResources/StandardMacros.IsValid` (`self.SequencePlayerActor`)
    (:`Is Valid`
      (switch `/Game/InteractionSystem/Blueprints/Connections/SequencePlayer/SequencePlayMode` (`self.PlayMode`)
        (:`NewEnumerator0`
          (if _returnvalue
            (`MovieSceneSequencePlayer.Play` _sequenceplayer :!label _label_2)
            (else
              (`MovieSceneSequencePlayer.PlayReverse` _sequenceplayer :!label _label_3))))
        (:`NewEnumerator1`
          (if _returnvalue
            (goto _label_3)
            (else
              (goto _label_2))))
        (:`NewEnumerator2`
          (goto _label_2))))))

(event `self.Off`
  (bind _sequenceplayer (`LevelSequenceActor.SequencePlayer` (`self.SequencePlayerActor`)))
  (`parent.Off`)
  (`/Engine/EditorBlueprintResources/StandardMacros.IsValid` (`self.SequencePlayerActor`)
    (:`Is Valid`
      (switch `/Game/InteractionSystem/Blueprints/Connections/SequencePlayer/SequencePlayMode` (`self.PlayMode`)
        (:`NewEnumerator0`
          (if (`MovieSceneSequencePlayer.IsReversed` _sequenceplayer)
            (`MovieSceneSequencePlayer.Play` _sequenceplayer)
            (else
              (`MovieSceneSequencePlayer.PlayReverse` _sequenceplayer))))
        (:`NewEnumerator1`
          (`MovieSceneSequencePlayer.Pause` _sequenceplayer))))))

(fn `UserConstructionScript`
  (`parent.UserConstructionScript`))