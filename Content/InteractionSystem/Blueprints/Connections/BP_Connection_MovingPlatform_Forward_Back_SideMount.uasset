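; Interaction-system connection for a side-mounted platform that travels out to a Destination offset and back according to its State.
; Tick advances or rewinds a clamped timer to lerp the platform at constant MoveSpeed, with paired DoOnce nodes toggling an electric hum between moving and arrived.
; The construction script places the target marker and laser beam end from Destination, then scales and side-offsets the mesh from PlatformSize.
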(event `self.ReceiveBeginPlay`
  (`parent.ReceiveBeginPlay`))

(event `self.ReceiveTick`
  (params (DeltaSeconds :type "Float (single-precision)"))
  (bind _electrichum (`self.ElectricHum`))
  (bind _output_get (set `self.ElaspedTime` (`KismetMathLibrary.FClamp` (+ (* DeltaSeconds (`KismetMathLibrary.SelectFloat` 1.0 -1.0 (`self.State`))) (`self.ElaspedTime`)) 0.0 (/ (`KismetMathLibrary.VSize` (`self.Destination`)) (`self.MoveSpeed`)))))
  (bind _returnvalue (/ (* _output_get (`self.MoveSpeed`)) (`KismetMathLibrary.VSize` (`self.Destination`))))
  (`SceneComponent.K2_SetRelativeLocation` (`self.Platform`) (`KismetMathLibrary.VLerp` (0.0 0.0 0.0) (`self.Destination`) _returnvalue) false false)
  (if (!= (`KismetMathLibrary.FTrunc` (* _returnvalue 10.0)) (`KismetMathLibrary.SelectFloat` 10.0 0.0 (`self.State`)))
    (`/Engine/EditorBlueprintResources/StandardMacros.DoOnce` false :!label _label
      (:`Completed`
        (`AudioComponent.Play` _electrichum 0.0)
        (goto _label_2 :!via `Reset`)))
    (else
      (`/Engine/EditorBlueprintResources/StandardMacros.DoOnce` false :!label _label_2
        (:`Completed`
          (`AudioComponent.Stop` _electrichum)
          (goto _label :!via `Reset`))))))

(event `self.On`
  (`parent.On`))

(event `self.Off`
  (`parent.Off`))

(fn `UserConstructionScript`
  (bind _platformsize_x (`KismetMathLibrary.BreakVector` (`self.PlatformSize`)))
  (bind (_platformsize_x_2 _platformsize_y) (`KismetMathLibrary.BreakVector` (`self.PlatformSize`)))
  (bind (_platformsize_x_3 _platformsize_y_2) (`KismetMathLibrary.BreakVector` (`self.PlatformSize`)))
  (bind (_relativelocation_x _relativelocation_y _relativelocation_z) (`KismetMathLibrary.BreakVector` (`SceneComponent.RelativeLocation` (`self.PlatformMesh`))))
  (`parent.UserConstructionScript`)
  (`SceneComponent.K2_SetRelativeLocation` (`self.Target`) (`self.Destination`) false false)
  (`NiagaraComponent.SetVariableVec3` (`self.LaserBeam`) "BeamEndLocation" (+ (`self.K2_GetActorLocation`) (`self.Destination`)))
  (`SceneComponent.SetWorldScale3D` (`self.PlatformMesh`) (`KismetMathLibrary.MakeVector` (/ (* _platformsize_x_2 2.0) 300.0) (/ (* _platformsize_y 2.0) 300.0) 1.0))
  (set `self.PlatformSize` (`KismetMathLibrary.MakeVector` _platformsize_x_3 _platformsize_y_2 _relativelocation_z))
  (`SceneComponent.K2_SetRelativeLocation` (`self.PlatformMesh`) (`KismetMathLibrary.MakeVector` (+ _platformsize_x 50.0)) false false))