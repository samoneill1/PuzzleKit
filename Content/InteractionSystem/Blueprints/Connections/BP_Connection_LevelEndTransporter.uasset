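; A connection-system transporter that ends the level when the player enters it while it is powered on.
; On and Off swap the Base and Cap grid materials and bind or unbind the PlayerDetection overlap, with Off staying on if CheckInputs returns true.
; An overlapping BP_FPS_Character receives LevelEnd with this actor.
; EndLevel is a placeholder that only prints a message instead of loading the next level.
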(event `self.ReceiveBeginPlay`)

(event `self.On`
  (set `self.State` true :!label _label)
  (`PrimitiveComponent.SetMaterial` (`self.Base`) 0 "/Game/InteractionSystem/Assets/Materials/ProcGrid/MI_ProcGrid_OnLines.MI_ProcGrid_OnLines")
  (`PrimitiveComponent.SetMaterial` (`self.Cap`) 0 "/Game/InteractionSystem/Assets/Materials/ProcGrid/MI_ProcGrid_OnLines.MI_ProcGrid_OnLines")
  (add `PrimitiveComponent.OnComponentBeginOverlap` (`self.  PlayerDetection`) (delegate `OverlapOnlyWhenOn`)))

(event `self.Off`
  (bind _returnstate (`self.CheckInputs`))
  (if _returnstate
    (goto _label)
    (else
      (set `self.State` false)
      (`PrimitiveComponent.SetMaterial` (`self.Base`) 0 "/Game/InteractionSystem/Assets/Materials/ProcGrid/MI_ProcGrid_OffLines.MI_ProcGrid_OffLines")
      (`PrimitiveComponent.SetMaterial` (`self.Cap`) 0 "/Game/InteractionSystem/Assets/Materials/ProcGrid/MI_ProcGrid_OffLines.MI_ProcGrid_OffLines")
      (clear `PrimitiveComponent.OnComponentBeginOverlap` (`self.  PlayerDetection`)))))

(event `OverlapOnlyWhenOn`
  (params (OverlappedComponent :type "PrimitiveComponent Object Reference") (OtherActor :type "Actor Object Reference") (OtherComp :type "PrimitiveComponent Object Reference") (OtherBodyIndex :type Integer) (bFromSweep :type Boolean) (SweepResult :type "HitResult Structure (by ref)"))
  (bind _asbp_fps_character (cast `/Game/InteractionSystem/Blueprints/Player/BP_FPS_Character` OtherActor))
  (`/Game/InteractionSystem/Blueprints/Player/BP_FPS_Character.LevelEnd` _asbp_fps_character self))

(event `/Game/InteractionSystem/Core/LevelEnd.EndLevel`
  (`KismetSystemLibrary.PrintString` "Should be loading next level!"))

(fn `UserConstructionScript`)