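; Interaction-system connection actor for a platform that slides forward to a Destination offset while its State is on, and back while off.
; Tick ramps a clamped elapsed time up or down by State, then lerps the platform's relative location at constant MoveSpeed, so it can reverse mid-travel.
; The construction script places the target and laser beam end from Destination and scales the mesh from PlatformSize.
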(event `self.ReceiveTick`
  (params (DeltaSeconds :type "Float (single-precision)"))
  (bind _output_get (set `self.ElaspedTime` (`KismetMathLibrary.FClamp` (+ (* DeltaSeconds (`KismetMathLibrary.SelectFloat` 1.0 -1.0 (`self.State`))) (`self.ElaspedTime`)) 0.0 (/ (`KismetMathLibrary.VSize` (`self.Destination`)) (`self.MoveSpeed`)))))
  (`SceneComponent.K2_SetRelativeLocation` (`self.Platform`) (`KismetMathLibrary.VLerp` (0.0 0.0 0.0) (`self.Destination`) (/ (* _output_get (`self.MoveSpeed`)) (`KismetMathLibrary.VSize` (`self.Destination`)))) false false))

(event `self.On`
  (`parent.On`))

(event `self.Off`
  (`parent.Off`))

(fn `UserConstructionScript`
  (bind (_platformsize_x _platformsize_y) (`KismetMathLibrary.BreakVector` (`self.PlatformSize`)))
  (bind (_platformsize_x_2 _platformsize_y_2) (`KismetMathLibrary.BreakVector` (`self.PlatformSize`)))
  (bind (_relativelocation_x _relativelocation_y _relativelocation_z) (`KismetMathLibrary.BreakVector` (`SceneComponent.RelativeLocation` (`self.PlatformMesh`))))
  (`parent.UserConstructionScript`)
  (`SceneComponent.K2_SetRelativeLocation` (`self.Target`) (`self.Destination`) false false)
  (`NiagaraComponent.SetVariableVec3` (`self.LaserBeam`) "BeamEndLocation" (+ (`self.K2_GetActorLocation`) (`self.Destination`)))
  (`SceneComponent.SetWorldScale3D` (`self.PlatformMesh`) (`KismetMathLibrary.MakeVector` (/ (* _platformsize_x 2.0) 300.0) (/ (* _platformsize_y 2.0) 300.0) 1.0))
  (set `self.PlatformSize` (`KismetMathLibrary.MakeVector` _platformsize_x_2 _platformsize_y_2 _relativelocation_z)))