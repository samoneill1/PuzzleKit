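; BP_Connection_Lightbar is an interaction-system connection actor, a lightbar that shows its on/off state through its glow.
; BeginPlay, On, Off and SyncInputState all route into UpdateState, with SyncInputState first storing the incoming State.
; UpdateState calls the parent version, then creates a dynamic material instance on Mesh slot 0 from the glow-on or glow-off material according to State.
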(event `self.ReceiveBeginPlay`
  (`parent.ReceiveBeginPlay`)
  (`self.Update State`))

(event `self.On`
  (`parent.On`)
  (`self.Update State`))

(event `self.Off`
  (`parent.Off`)
  (`self.Update State`))

(event `/Game/InteractionSystem/Core/BPI_Interaction.Sync Input State`
  (params (State :type Boolean))
  (set `self.State` State)
  (`self.Update State`))

(fn `Get Fracture Bool`
  (returns (IsFracture :type Boolean))
  (return false))

(fn `Get Item Type`
  (returns (`Item Type` :type "/Game/InteractionSystem/Core/E_ItemType Enum"))
  (return "NewEnumerator0"))

(fn `Get Mesh`
  (returns (Mesh :type "PrimitiveComponent Object Reference"))
  (return null))

(fn `Update State`
  (`parent.Update State`)
  (`PrimitiveComponent.CreateDynamicMaterialInstance` (`self.Mesh`) 0 (select `bool` (`self.State`) :`false` "/Game/InteractionSystem/Assets/Materials/Glow/MI_Glow_Off.MI_Glow_Off" :`true` "/Game/InteractionSystem/Assets/Materials/Glow/MI_Glow_On.MI_Glow_On" :!type "MaterialInterface Object Reference") "None"))

(fn `UserConstructionScript`
  (`parent.UserConstructionScript`))