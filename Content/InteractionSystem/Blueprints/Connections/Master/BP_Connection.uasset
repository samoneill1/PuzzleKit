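; BP_Connection is the master Blueprint for devices driven by BP_Input actors in the interaction system, holding a boolean State.
; On BeginPlay it scans all inputs for connections targeting itself, caching each with its Invert flag.
; On sets State true directly, while Off recomputes it through CheckInputs, which returns true if any input's State equals its Invert value.
; UpdateState is an empty function.
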(event `self.ReceiveBeginPlay`
  ;[1 1 1] On BeginPlay, grad all inputs that target this device
  (bind _outactors (`GameplayStatics.GetAllActorsOfClass` "/Game/InteractionSystem/Blueprints/Input/Master/BP_Input.BP_Input_C"))
  (for _array_element _outactors
    (for _array_element_2 (`/Game/InteractionSystem/Blueprints/Input/Master/BP_Input.Connection2` _array_element)
      (if (== (break `/Game/InteractionSystem/Blueprints/Input/Master/Connection` _array_element_2) self)
        (`KismetArrayLibrary.Array_Add` (`self.InputsTargettingMe`) _array_element)
        (`BlueprintMapLibrary.Map_Add` (`self.Invert`) _array_element (`.Invert_8_01B3B2A949047C48E4B5FEBB83D663A9` (break `/Game/InteractionSystem/Blueprints/Input/Master/Connection` _array_element_2)))))))

(event `On`
  (set `self.State` true))

(event `Off`
  (bind _returnstate (`self.CheckInputs`))
  (set `self.State` _returnstate))

(fn `CheckInputs`
  (returns (ReturnState :type Boolean))
  (locals (LocalState :type Boolean))
  (set `local.LocalState` false)
  (for _array_element (`self.InputsTargettingMe`)
    (if (== (`BlueprintMapLibrary.Map_Find` (`self.Invert`) _array_element) (`/Game/InteractionSystem/Blueprints/Input/Master/BP_Input.State` _array_element))
      (set `local.LocalState` true)))
  (return (`local.LocalState`)))

(fn `Update State`)

(fn `UserConstructionScript`)