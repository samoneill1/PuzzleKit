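; Force field connection for the interaction system, a yellow barrier between two pillars that ignores two custom collision channels (ALLOWBLOCKS variant).
; The construction script positions and scales both frames from the pillar and height variables, then generates a procedural box mesh spanning them, with collision and a dynamic material.
; On and Off call the parent events and toggle only the mesh's visibility, leaving collision untouched.
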(event `self.On`
  (`parent.On`)
  (`SceneComponent.SetVisibility` (`self.ForcefieldMesh`) true false))

(event `self.Off`
  (`parent.Off`)
  (`SceneComponent.SetVisibility` (`self.ForcefieldMesh`) false false))

(fn `UserConstructionScript`
  (bind _frame_l (`self.Frame_L`))
  (bind _frame_r (`self.Frame_R`))
  (bind (_right_pillar_x _right_pillar_y) (`KismetMathLibrary.BreakVector` (`self.Right_Pillar`)))
  (bind (_height_x _height_y _height_z) (`KismetMathLibrary.BreakVector` (`self.Height`)))
  (bind (_left_pillar_x _left_pillar_y) (`KismetMathLibrary.BreakVector` (`self.Left_Pillar`)))
  (bind (_right_pillar_x_2 _right_pillar_y_2) (`KismetMathLibrary.BreakVector` (`self.Right_Pillar`)))
  (bind (_height_x_2 _height_y_2 _height_z_2) (`KismetMathLibrary.BreakVector` (`self.Height`)))
  (bind (_left_pillar_x_2 _left_pillar_y_2) (`KismetMathLibrary.BreakVector` (`self.Left_Pillar`)))
  (bind _returnvalue (/ _height_z_2 2.0))
  (bind _returnvalue_2 (/ _height_z_2 220.0))
  (bind _returnvalue_3 (/ _height_z 2.0))
  (bind _relativelocation (`SceneComponent.RelativeLocation` _frame_l))
  (bind _relativelocation_2 (`SceneComponent.RelativeLocation` _frame_r))
  (bind (_returnvalue_x _returnvalue_y) (`KismetMathLibrary.BreakVector` (- _relativelocation (/ (- _relativelocation _relativelocation_2) (2.0 2.0 2.0)))))
  (`parent.UserConstructionScript`)
  (set `self.Left_Pillar` (`KismetMathLibrary.MakeVector` _left_pillar_x_2 _left_pillar_y_2 _returnvalue_3))
  (set `self.Right_Pillar` (`KismetMathLibrary.MakeVector` _right_pillar_x _right_pillar_y _returnvalue_3))
  (`SceneComponent.K2_SetRelativeLocation` (`self.Frame_L`) (`KismetMathLibrary.MakeVector` _left_pillar_x _left_pillar_y) false false)
  (`SceneComponent.K2_SetRelativeLocation` (`self.Frame_R`) (`KismetMathLibrary.MakeVector` _right_pillar_x_2 _right_pillar_y_2) false false)
  (`SceneComponent.SetRelativeScale3D` _frame_r (`KismetMathLibrary.MakeVector` 1.0 1.0 _returnvalue_2))
  (`SceneComponent.SetRelativeScale3D` _frame_l (`KismetMathLibrary.MakeVector` 1.0 1.0 _returnvalue_2))
  (bind (_vertices _triangles _normals _uvs _tangents) (`KismetProceduralMeshLibrary.GenerateBoxMesh` (`KismetMathLibrary.MakeVector` 1.0 (/ (`KismetMathLibrary.Vector_Distance` _relativelocation _relativelocation_2) 2.0) _returnvalue)))
  (set `self.Height` (`KismetMathLibrary.MakeVector` _returnvalue_x _returnvalue_y _height_z_2))
  (bind _returnvalue_4 (`AddComponent|NODE_AddProceduralMeshComponent-0` :`RelativeTransform` (`KismetMathLibrary.MakeTransform` (`KismetMathLibrary.MakeVector` _returnvalue_x _returnvalue_y _returnvalue))))
  (bind _output_get (set `self.ForcefieldMesh` _returnvalue_4))
  (`SceneComponent.K2_SetRelativeRotation` _output_get (`KismetMathLibrary.ComposeRotators` (`KismetMathLibrary.FindLookAtRotation` (`SceneComponent.RelativeLocation` (`self.Frame_L`)) (`SceneComponent.RelativeLocation` (`self.Frame_R`))) (struct :`Yaw` 90.0)) false false)
  (`ProceduralMeshComponent.CreateMeshSection_LinearColor` :`self` _output_get :`Vertices` _vertices :`Triangles` _triangles :`Normals` _normals :`UV0` _uvs :`Tangents` _tangents :`bCreateCollision` true)
  (`PrimitiveComponent.SetCollisionResponseToChannel` (`self.ForcefieldMesh`) "ECC_GameTraceChannel2" "ECR_Ignore")
  (`PrimitiveComponent.SetCollisionResponseToChannel` (`self.ForcefieldMesh`) "ECC_GameTraceChannel1" "ECR_Ignore")
  (bind _returnvalue_5 (`KismetMaterialLibrary.CreateDynamicMaterialInstance` "/Game/InteractionSystem/Blueprints/Connections/Forcefield_M.Forcefield_M"))
  (bind _output_get_2 (set `self.ForcefieldMaterial` _returnvalue_5))
  (`PrimitiveComponent.SetMaterial` (`self.ForcefieldMesh`) 0 _output_get_2)
  (`MaterialInstanceDynamic.SetVectorParameterValue` _output_get_2 "Colour" (struct :`R` 1.0 :`G` 1.0 :`A` 1.0)))