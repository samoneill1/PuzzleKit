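; Side-mounted moving platform connection that shuttles back and forth between its origin and Destination while switched on.
; Tick runs a clamped timer that reverses at each end and lerps the platform at MoveSpeed, holding position while State is off.
; DoOnce gates start the electric hum during travel and stop it at the far end.
; The construction script places the target and laser beam end, then scales and side-offsets the mesh from PlatformSize.
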(event `self.ReceiveTick`
  (params (DeltaSeconds :type "Float (single-precision)"))
  (bind _electrichum (`self.ElectricHum`))
  (bind _returnvalue (/ (`KismetMathLibrary.VSize` (`self.Destination`)) (`self.MoveSpeed`)))
  (if (`self.State`)
    (bind _output_get (set `self.ElaspedTime` (`KismetMathLibrary.FClamp` (+ (* DeltaSeconds (`KismetMathLibrary.SelectFloat` 1.0 -1.0 (`self.Forwards`))) (`self.ElaspedTime`)) 0.0 _returnvalue)))
    (if (== _output_get _returnvalue)
      (set `self.Forwards` false)
      (elif (== _output_get 0.0)
        (set `self.Forwards` true)))
    (bind _returnvalue_2 (/ (* _output_get (`self.MoveSpeed`)) (`KismetMathLibrary.VSize` (`self.Destination`))))
    (`SceneComponent.K2_SetRelativeLocation` (`self.Platform`) (`KismetMathLibrary.VLerp` (0.0 0.0 0.0) (`self.Destination`) _returnvalue_2) false false)
    (if (!= (`KismetMathLibrary.FTrunc` (* _returnvalue_2 10.0)) (`KismetMathLibrary.SelectFloat` 10.0 0.0 (`self.State`)))
      (`/Engine/EditorBlueprintResources/StandardMacros.DoOnce` false :!label _label
        (:`Completed`
          (`AudioComponent.Play` _electrichum 0.0)
          (goto _label_2 :!via `Reset`)))
      (else
        (`/Engine/EditorBlueprintResources/StandardMacros.DoOnce` false :!label _label_2
          (:`Completed`
            (`AudioComponent.Stop` _electrichum)
            (goto _label :!via `Reset`)))))))

(event `self.On`
  (`parent.On`))

(event `self.Off`
  (`parent.Off`))

(fn `UserConstructionScript`
  (bind _platformsize_x (`KismetMathLibrary.BreakVector` (`self.PlatformSize`)))
  (bind _platformsize_x_2 (`KismetMathLibrary.BreakVector` (`self.PlatformSize`)))
  (bind (_platformsize_x_3 _platformsize_y) (`KismetMathLibrary.BreakVector` (`self.PlatformSize`)))
  (bind (_platformsize_x_4 _platformsize_y_2) (`KismetMathLibrary.BreakVector` (`self.PlatformSize`)))
  (bind (_relativelocation_x _relativelocation_y _relativelocation_z) (`KismetMathLibrary.BreakVector` (`SceneComponent.RelativeLocation` (`self.PlatformMesh`))))
  (`parent.UserConstructionScript`)
  (`SceneComponent.K2_SetRelativeLocation` (`self.Target`) (`self.Destination`) false false)
  (`NiagaraComponent.SetVariableVec3` (`self.LaserBeam`) "BeamEndLocation" (+ (`self.K2_GetActorLocation`) (`self.Destination`)))
  (`SceneComponent.SetWorldScale3D` (`self.PlatformMesh`) (`KismetMathLibrary.MakeVector` (/ (* _platformsize_x_3 2.0) 300.0) (/ (* _platformsize_y 2.0) 300.0) 1.0))
  (set `self.PlatformSize` (`KismetMathLibrary.MakeVector` _platformsize_x_4 _platformsize_y_2 _relativelocation_z))
  (`SceneComponent.K2_SetRelativeLocation` (`self.PlatformMesh`) (`KismetMathLibrary.MakeVector` (+ _platformsize_x_2 50.0)) false false)
  (`SceneComponent.K2_SetRelativeLocation` (`self.PlatformMesh`) (`KismetMathLibrary.MakeVector` (+ _platformsize_x 50.0)) false false))